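; BP_Helpers is a Blueprint helper asset whose GetPointGrid function builds an array of evenly spaced 3D points on a horizontal plane.
; Nested X and Y loops scale indices by per-axis spacing, offset them by a center at constant Z, and can negate the Y offset.
; Indices start at zero or straddle the center; centered mode yields one more point per axis than the sample count, as its bounds are inclusive.
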(fn `GetPointGrid`
  (params (SampleCountX :type Integer) (SpacingX :type "Float (double-precision)") (CenterX :type "Float (double-precision)") (SampleCountY :type Integer) (SpacingY :type "Float (double-precision)") (CenterY :type "Float (double-precision)") (Z :type "Float (double-precision)") (InvertYAxis :type Boolean) (Centered :type Boolean))
  (returns (PointGrid :type "Array of Vector Structure"))
  (locals (X :type "Float (double-precision)") (Y :type "Float (double-precision)") (Grid :type "Array of Vector Structure") (FirstIndexX :type Integer) (LastIndexX :type Integer) (FirstIndexY :type Integer) (LastIndexY :type Integer) (OffsetX :type "Float (double-precision)") (OffsetY :type "Float (double-precision)"))
  (bind _samplecountx (`local.SampleCountX`))
  (bind _samplecounty (`local.SampleCountY`))
  (if Centered
    ;[1 1 1] Compute centered indices
    (bind _output_get (set `local.FirstIndexX` (/ _samplecountx -2)))
    (set `local.LastIndexX` (+ _samplecountx _output_get))
    (bind _output_get_2 (set `local.FirstIndexY` (/ _samplecounty -2)))
    (set `local.LastIndexY` (+ _output_get_2 _samplecounty))
    (else
      ;[1 1 1] Compute 0-bases indices
      (set `local.FirstIndexX` 0)
      (set `local.LastIndexX` (- (`local.SampleCountX`) 1))
      (set `local.FirstIndexY` 0)
      (set `local.LastIndexY` (- (`local.SampleCountY`) 1))))
  ;[1 1 1] Compute X
  (for _index (range (`local.FirstIndexX`) (+ (`local.LastIndexX`) 1))
    (set `local.X` (* _index (`local.SpacingX`)))
    ;[1 1 1] Set Y
    (for _index_2 (range (`local.FirstIndexY`) (+ (`local.LastIndexY`) 1))
      (if (`local.InvertYAxis`)
        (bind _returnvalue (* _index_2 (`local.SpacingY`)))
        (set `local.Y` (* _returnvalue -1.0))
        (else
          (set `local.Y` _returnvalue)))
      ;[1 1 1] Add to grid
      (`KismetArrayLibrary.Array_Add` (`local.Grid`) (`KismetMathLibrary.MakeVector` (+ (`local.CenterX`) (`local.X`)) (+ (`local.CenterY`) (`local.Y`)) (`local.Z`)))))
  (return (`local.Grid`)))