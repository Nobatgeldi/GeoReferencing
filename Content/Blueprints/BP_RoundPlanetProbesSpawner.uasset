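; BP_RoundPlanetProbesSpawner scatters BP_LocationProbe actors over a latitude/longitude grid on a georeferenced round planet.
; SpawnProbes centers the grid on either the GeoReferencing origin or custom coordinates, with configurable count and degree spacing.
; Each point becomes a tangent transform from the GeoReferencing System, orienting the scaled probe to the planet's curvature.
; RemoveProbes destroys every BP_LocationProbe found in the world, not only those this spawner created.
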(event `self.ReceiveBeginPlay`)

(fn `RemoveProbes`
  (bind _outactors (`GameplayStatics.GetAllActorsOfClass` "/GeoReferencing/Models/LocationProbe/BP_LocationProbe.BP_LocationProbe_C"))
  (for _array_element _outactors
    (`self.K2_DestroyActor` _array_element)))

(fn `SpawnProbes`
  (locals (GeoReferencingSystem :type "GeoReferencingSystem Object Reference") (CenterX :type "Float (double-precision)" :default 0.0) (CenterY :type "Float (double-precision)" :default 0.0) (CenterZ :type "Float (double-precision)" :default 0.0))
  (bind _probesscale (`self.ProbesScale`))
  (bind _georeferencingsystem (`local.GeoReferencingSystem`))
  ;[1 1 1] Grab GeoReferencing System
  (set `local.GeoReferencingSystem` (`GeoReferencingSystem.GetGeoReferencingSystem`))
  ;[1 1 1] Compute Start Origin
  (if (`self.UseOriginAsCenter`)
    (set `local.CenterX` (`GeoReferencingSystem.OriginLatitude` _georeferencingsystem))
    (set `local.CenterY` (`GeoReferencingSystem.OriginLongitude` _georeferencingsystem))
    (set `local.CenterZ` (`GeoReferencingSystem.OriginAltitude` _georeferencingsystem))
    (else
      (set `local.CenterX` (`self.CenterLatitude`))
      (set `local.CenterY` (`self.CenterLongitude`))
      (set `local.CenterZ` (`self.CenterAltitude`))))
  ;[1 1 1] Iterate on a grid of Geographic Coordinates
  (bind _pointgrid (`/GeoReferencing/Blueprints/BP_Helpers.GetPointGrid` (- (`self.CountLat`) 1) (`self.SpacingLat (Deg)`) (`local.CenterX`) (- (`self.CountLong`) 1) (`self.SpacingLong (Deg)`) (`local.CenterY`) (`local.CenterZ`) false true))
  (for _array_element _pointgrid
    ;[1 1 1] Spawn Probe
    (bind _returnvalue (`GeoReferencingSystem.GetTangentTransformAtGeographicLocation` (`local.GeoReferencingSystem`) (`GeographicCoordinatesFunctionLibrary.MakeGeographicCoordinates` _array_element)))
    (`|SpawnActorFromClass` "/GeoReferencing/Models/LocationProbe/BP_LocationProbe.BP_LocationProbe_C" (`KismetMathLibrary.MakeTransform` (.location _returnvalue) (.rotation _returnvalue) (`KismetMathLibrary.MakeVector` _probesscale _probesscale _probesscale)) "Undefined" "OverrideRootScale" null null)))

(fn `UserConstructionScript`)