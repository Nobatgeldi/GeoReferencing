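; Example actor that places itself at a latitude, longitude and altitude using the GeoReferencing plugin.
; Its construction script takes the first GeoReferencingSystem in the level and, if valid, converts the Latitude, Longitude and Altitude properties to an engine tangent transform.
; It then sets the actor's location and rotation from that transform; the event graph holds only disabled stub events.
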(fn `UserConstructionScript`
  ;[1 1 1] Get a Valid Georeferencing System
  (bind _outactors (`GameplayStatics.GetAllActorsOfClass` "/Script/GeoReferencing.GeoReferencingSystem"))
  (if (`KismetArrayLibrary.Array_IsNotEmpty` _outactors)
    (bind _output (`|GetArrayItem` _outactors))
    (`/Engine/EditorBlueprintResources/StandardMacros.IsValid` _output
      (:`Is Valid`
        ;[1 1 1] Convert the Lat/Long/Alt properties to Engine Coordinates
        (bind _returnvalue (`GeoReferencingSystem.GetTangentTransformAtGeographicLocation` _output (`GeographicCoordinatesFunctionLibrary.MakeGeographicCoordinates` (`KismetMathLibrary.MakeVector` (`self.Latitude`) (`self.Longitude`) (`self.Altitude`)))))
        ;[1 1 1] Update Actor Location and Rotation
        (`self.K2_SetActorLocationAndRotation` (.location _returnvalue) (.rotation _returnvalue))))))