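; BP_LocationProbe is a probe actor that shows the local East, North and Up directions at its position using the GeoReferencing system.
; The construction script converts the actor location to ECEF, fetches the ENU vectors there and orients three arrows along them.
; Both the construction script and BeginPlay register the actor as ParentActor of its UMG_ProbeText widget.
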(event `self.ReceiveBeginPlay`
  ;[1 1 1] Register myself to the widget
  (bind _asumg_probe_text (cast `/GeoReferencing/Models/LocationProbe/UMG_ProbeText` (`WidgetComponent.GetWidget` (`self.LocationWidget`))))
  (set `/GeoReferencing/Models/LocationProbe/UMG_ProbeText.ParentActor` self _asumg_probe_text))

(fn `UserConstructionScript`
  (bind _returnvalue (`KismetMathLibrary.Vector_Zero`))
  ;[1 1 1] Register to Parent Widget
  (bind _asumg_probe_text (cast `/GeoReferencing/Models/LocationProbe/UMG_ProbeText` (`WidgetComponent.GetWidget` (`self.LocationWidget`))))
  (set `/GeoReferencing/Models/LocationProbe/UMG_ProbeText.ParentActor` self _asumg_probe_text)
  ;[1 1 1] Compute ENU Vectors
  (bind _ecefcoordinates (`GeoReferencingSystem.K2_EngineToECEF` (`GeoReferencingSystem.GetGeoReferencingSystem`) (`self.K2_GetActorLocation`)))
  (bind (_east _north _up) (`GeoReferencingSystem.K2_GetENUVectorsAtECEFLocation` (`GeoReferencingSystem.GetGeoReferencingSystem`) _ecefcoordinates))
  ;[1 1 1] Update Arrows transformation
  (`SceneComponent.K2_SetWorldRotation` (`self.ArrowEast`) (`KismetMathLibrary.MakeRotationFromAxes` _east) false false)
  (`SceneComponent.K2_SetWorldRotation` (`self.ArrowNorth`) (`KismetMathLibrary.FindLookAtRotation` _returnvalue _north) false false)
  (`SceneComponent.K2_SetWorldRotation` (`self.ArrowUp`) (`KismetMathLibrary.FindLookAtRotation` _returnvalue _up) false false))